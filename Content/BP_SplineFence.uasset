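; Spline-driven fence actor that lays copies of a fence mesh along an editable spline in the construction script.
; It divides the spline length by the mesh's X-axis bound to get the segment count, adding a blocking-collision spline mesh component for each.
; Segment endpoints are sampled by distance, with tangents normalized and scaled to mesh length; any leftover length stays uncovered.
; A debug print shows the last segment index, and the event graph is empty.
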(event EventBeginPlay)

(event Collision|EventActorBeginOverlap
  (params (OtherActor :type Actor%20Object%20Reference)))

(event EventTick
  (params (DeltaSeconds :type Float%20%28single-precision%29)))

(fn ConstructionScript
  (bind _spline (Variables|Default|GetSpline))
  (bind _fencemesh (Variables|Default|GetFenceMesh))
  (bind _spline_2 (Variables|Default|GetSpline))
  (bind _returnvalue (StaticMesh|GetBoundingBox _fencemesh))
  (bind _returnvalue_2 (Spline|GetSplineLength _spline))
  (bind _returnvalue_3 (- (.x (.max _returnvalue)) (.x (.min _returnvalue))))
  (bind _returnvalue_4 (/ _returnvalue_2 _returnvalue_3))
  (bind _returnvalue_5 (Math|Float|Truncate _returnvalue_4))
  (bind _returnvalue_6 (- _returnvalue_5 1))
  (Variables|Default|SetMeshLength _returnvalue_3)
  (for _index (range 0 _returnvalue_6)
    (bind _returnvalue_7 (AddComponent|AddSplineMeshComponent false))
    (Collision|SetCollisionProfileName _returnvalue_7 "BlockAll" true :!class /Script/Engine.PrimitiveComponent)
    (Components|StaticMesh|SetStaticMesh _returnvalue_7 (Variables|Default|GetFenceMesh))
    (SplineMesh|SetForwardAxis _returnvalue_7 (Variables|Default|GetForwardAxis) true)
    (SplineMesh|SetStartandEnd _returnvalue_7 (Spline|GetLocationatDistanceAlongSpline _spline_2 (Math|Conversions|ToFloat(Integer) (* _index (Variables|Default|GetMeshLength))) "Local") (* (Math|Vector|Normalize (Spline|GetTangentatDistanceAlongSpline _spline_2 (Math|Conversions|ToFloat(Integer) (* _index (Variables|Default|GetMeshLength))) "Local")) (Variables|Default|GetMeshLength)) (Spline|GetLocationatDistanceAlongSpline _spline_2 (Math|Conversions|ToFloat(Integer) (* (+ _index 1) (Variables|Default|GetMeshLength))) "Local") (* (Math|Vector|Normalize (Spline|GetTangentatDistanceAlongSpline _spline_2 (Math|Conversions|ToFloat(Integer) (* (+ _index 1) (Variables|Default|GetMeshLength))) "Local")) (Variables|Default|GetMeshLength)) true :!class /Script/Engine.SplineMeshComponent))
  (Development|PrintString (Utilities|String|ToString(Integer) _returnvalue_6)))